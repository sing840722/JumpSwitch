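; Touchable platform actor that moves along world X and lets the player jump to it by teleport.
; Construction adds a static mesh component with a randomly picked coloured building mesh.
; PlatFallingSpeed is copied from GameState_BP at construction and BeginPlay, then added to X every Tick without delta-time scaling.
; Touching the platform teleports the controlled Player_Char to 200 units above it.
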(event `self.ReceiveBeginPlay`
  (`self.GetFallingSpeed`))

(event `self.ReceiveActorBeginOverlap`
  (params (OtherActor :type "Actor Object Reference")))

(event `self.ReceiveTick`
  (params (DeltaSeconds :type "Float (single-precision)"))
  (`self.K2_SetActorLocation` (+ (`self.K2_GetActorLocation`) (`KismetMathLibrary.MakeVector` (`self.PlatFallingSpeed`)))))

(event `self.ReceiveActorOnInputTouchBegin`
  (params (FingerIndex :type "ETouchIndex Enum" :default "Touch1"))
  (bind _asplayer_char (cast `/Game/Blueprints/Player_Char` (`Controller.K2_GetPawn` (`GameplayStatics.GetPlayerController` 0))))
  (`self.K2_TeleportTo` :`self` _asplayer_char :`DestLocation` (+ (`self.K2_GetActorLocation`) (0.0 0.0 200.0))))

(fn `GetFallingSpeed`
  (bind _asgame_state_bp (cast `/Game/Blueprints/GameState_BP` (`GameplayStatics.GetGameState`)))
  (set `self.PlatFallingSpeed` (`/Game/Blueprints/GameState_BP.FallingSpeed` _asgame_state_bp)))

(fn `RandomColour`
  (bind _returnvalue (`AddComponent|Static Mesh Component_254` :`RelativeTransform` (`SceneComponent.GetSocketTransform` (`self.DefaultSceneRoot`) "None" "RTS_World")))
  (switch `int` (`KismetMathLibrary.RandomIntegerInRange` 0 3)
    (:`Default`
      (`StaticMeshComponent.SetStaticMesh` _returnvalue "/Game/Assets/Buildings/YELLOW_Building.YELLOW_Building" :!label _label))
    (:`0`
      (`StaticMeshComponent.SetStaticMesh` _returnvalue "/Game/Assets/Buildings/GREEN_Building.GREEN_Building"))
    (:`1`
      (`StaticMeshComponent.SetStaticMesh` _returnvalue "/Game/Assets/Buildings/Blue_Building.Blue_Building"))
    (:`2`
      (`StaticMeshComponent.SetStaticMesh` _returnvalue "/Game/Assets/Buildings/RED_Building.RED_Building"))
    (:`3`
      (goto _label))))

(fn `UserConstructionScript`
  (`self.RandomColour`)
  (`self.GetFallingSpeed`))