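; Game state Blueprint that extends rows of left and right buildings, apparently for endlessly scrolling scenery.
; SpawnNextRight and SpawnNextLeft spawn a building at a fixed negative X offset from the last array entry, resize the array to a fixed length, then append it.
; SpawnRightDup instead teleports a given actor to a positive X offset from the last right building, leaving the array untouched.
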(event `self.ReceiveBeginPlay`)

(event `self.ReceiveTick`
  (params (DeltaSeconds :type "Float (single-precision)")))

(fn `SpawnNextLeft`
  (bind _leftbuildingarray (`self.LeftBuildingArray`))
  (bind _leftbuildingarray_2 (`self.LeftBuildingArray`))
  (bind _item (`KismetArrayLibrary.Array_Get` _leftbuildingarray (`KismetArrayLibrary.Array_LastIndex` _leftbuildingarray)))
  (`/Engine/EditorBlueprintResources/StandardMacros.IsValid` _item
    (:`Is Valid`
      (bind _returnvalue (`|SpawnActorFromClass` "/Game/Blueprints/LeftBuildings_BP.LeftBuildings_BP_C" (`KismetMathLibrary.MakeTransform` (`KismetMathLibrary.MakeVector` (- (.x (.location (`self.GetTransform` _item))) 1200.0) (.y (.location (`self.GetTransform` _item))) (.z (.location (`self.GetTransform` _item)))) (.rotation (`self.GetTransform` _item)) (.scale (`self.GetTransform` _item))) "AlwaysSpawn" "OverrideRootScale"))
      (`KismetArrayLibrary.Array_Resize` _leftbuildingarray_2 10)
      (`KismetArrayLibrary.Array_Add` _leftbuildingarray_2 _returnvalue))))

(fn `SpawnNextRight`
  (bind _rightbuildingarray (`self.RightBuildingArray`))
  (bind _rightbuildingarray_2 (`self.RightBuildingArray`))
  (bind _item (`KismetArrayLibrary.Array_Get` _rightbuildingarray_2 (`KismetArrayLibrary.Array_LastIndex` _rightbuildingarray_2)))
  (`/Engine/EditorBlueprintResources/StandardMacros.IsValid` _item
    (:`Is Valid`
      (bind _returnvalue (`|SpawnActorFromClass` "/Game/Blueprints/RightBuildings_BP.RightBuildings_BP_C" (`KismetMathLibrary.MakeTransform` (`KismetMathLibrary.MakeVector` (- (.x (.location (`self.GetTransform` _item))) 1250.0) (.y (.location (`self.GetTransform` _item))) (.z (.location (`self.GetTransform` _item)))) (.rotation (`self.GetTransform` _item)) (.scale (`self.GetTransform` _item))) "AlwaysSpawn" "OverrideRootScale"))
      (`KismetArrayLibrary.Array_Resize` _rightbuildingarray 10)
      (`KismetArrayLibrary.Array_Add` _rightbuildingarray _returnvalue))))

(fn `SpawnRightDup`
  (params (NewParam :type "/Game/Blueprints/RightBuildings_BP Object Reference"))
  (bind _rightbuildingarray (`self.RightBuildingArray`))
  (bind _item (`KismetArrayLibrary.Array_Get` _rightbuildingarray (`KismetArrayLibrary.Array_LastIndex` _rightbuildingarray)))
  (bind (_returnvalue_location _returnvalue_rotation) (`KismetMathLibrary.BreakTransform` (`self.GetTransform` _item)))
  (`/Engine/EditorBlueprintResources/StandardMacros.IsValid` NewParam
    (:`Is Valid`
      (`/Engine/EditorBlueprintResources/StandardMacros.IsValid` _item
        (:`Is Valid`
          (`self.K2_TeleportTo` NewParam (`KismetMathLibrary.MakeVector` (- (.x _returnvalue_location) -3000.0) (.y _returnvalue_location) (.z _returnvalue_location)) _returnvalue_rotation))))))

(fn `UserConstructionScript`)