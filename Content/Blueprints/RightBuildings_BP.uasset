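; Tappable building for a colour-matching jumping game, randomised on construction.
; Random picks a coloured or black mesh, with GameState's Chance setting the range; coloured buildings either get a random prop or set their colour Id, not both.
; The first matching touch teleports the player onto it, adds score through GameState and GM2, and swaps to the used mesh.
; A colour mismatch on an unused building saves the score to the GameInstance and opens Defeat.
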(event `self.ReceiveTick`
  (params (DeltaSeconds :type "Float (single-precision)")))

(event `self.ReceiveActorOnInputTouchBegin`
  (params (FingerIndex :type "ETouchIndex Enum" :default "Touch1"))
  (bind (_returnvalue_x _returnvalue_y _returnvalue_z) (`KismetMathLibrary.BreakVector` (`self.K2_GetActorLocation`)))
  (bind _asgame_pc (cast `/Game/Blueprints/Game_PC` (`GameplayStatics.GetPlayerController` 0)))
  (if (== (`self.numOfJump`) 0)
    (bind _asgame_state_bp (cast `/Game/Blueprints/GameState_BP` (`GameplayStatics.GetGameState`)))
    (if (== (`/Game/Blueprints/Game_PC.CurrentColour` _asgame_pc) (`self.id`))
      (`/Engine/EditorBlueprintResources/StandardMacros.IncrementInt` (`self.numOfJump`)
        (:`  `
          (bind _asplayer_char (cast `/Game/Blueprints/Player_Char` (`Controller.K2_GetPawn` _asgame_pc)))
          (`self.K2_TeleportTo` :`self` _asplayer_char :`DestLocation` (`KismetMathLibrary.MakeVector` (+ _returnvalue_x 100.0) _returnvalue_y (+ _returnvalue_z 50.0)))
          (bind _asgm2 (cast `/Game/Blueprints/GM2` (`GameplayStatics.GetGameMode`)))
          (bind _output_get (set `/Game/Blueprints/GameState_BP.Score` (+ (`/Game/Blueprints/GameState_BP.Score` _asgame_state_bp) (`self.willScore`)) _asgame_state_bp))
          (`/Game/Blueprints/GM2.Scoring` _asgm2 _output_get)
          (`StaticMeshComponent.SetStaticMesh` (`self.StaticMesh`) "/Game/Assets/Buildings/Used_Building.Used_Building")
          (`GameplayStatics.PlaySound2D` "/Game/Sounds/Blop-Mark_DiAngelo-79054334.Blop-Mark_DiAngelo-79054334")))
      (else
        (bind _asmy_gi (cast `/Game/Blueprints/myGI` (`GameplayStatics.GetGameInstance`)))
        (set `/Game/Blueprints/myGI.Score` (`KismetMathLibrary.FTrunc` (`/Game/Blueprints/GameState_BP.Score` _asgame_state_bp)) _asmy_gi)
        (`GameplayStatics.OpenLevel` "Defeat")))))

(fn `Random`
  (bind _staticmesh (`self.StaticMesh`))
  (bind _asgame_state_bp (cast `/Game/Blueprints/GameState_BP` (`GameplayStatics.GetGameState`)))
  (switch `int` (`KismetMathLibrary.RandomIntegerInRange` 1 (`/Game/Blueprints/GameState_BP.chance` _asgame_state_bp))
    (:`Default`
      (`StaticMeshComponent.SetStaticMesh` _staticmesh "/Game/Assets/Buildings/Black_Building.Black_Building" :!label _label))
    (:`1`
      (`StaticMeshComponent.SetStaticMesh` _staticmesh "/Game/Assets/Buildings/GREEN_Building.GREEN_Building")
      (`self.SpawnParts`
        (:`true`
          (`self.RandomParts` :!label _label_2))
        (:`false`
          (set `self.id` 0))))
    (:`2`
      (`StaticMeshComponent.SetStaticMesh` _staticmesh "/Game/Assets/Buildings/YELLOW_Building.YELLOW_Building")
      (`self.SpawnParts`
        (:`true`
          (goto _label_2))
        (:`false`
          (set `self.id` 1))))
    (:`3`
      (`StaticMeshComponent.SetStaticMesh` _staticmesh "/Game/Assets/Buildings/YELLOW_Building.YELLOW_Building")
      (`self.SpawnParts`
        (:`true`
          (goto _label_2))
        (:`false`
          (set `self.id` 1))))
    (:`4`
      (`StaticMeshComponent.SetStaticMesh` _staticmesh "/Game/Assets/Buildings/RED_Building.RED_Building")
      (`self.SpawnParts`
        (:`true`
          (goto _label_2))
        (:`false`
          (set `self.id` 2))))
    (:`5`
      (`StaticMeshComponent.SetStaticMesh` _staticmesh "/Game/Assets/Buildings/RED_Building.RED_Building")
      (`self.SpawnParts`
        (:`true`
          (goto _label_2))
        (:`false`
          (set `self.id` 2))))
    (:`6`
      (`StaticMeshComponent.SetStaticMesh` _staticmesh "/Game/Assets/Buildings/Blue_Building.Blue_Building")
      (`self.SpawnParts`
        (:`true`
          (goto _label_2))
        (:`false`
          (set `self.id` 3))))
    (:`7`
      (`StaticMeshComponent.SetStaticMesh` _staticmesh "/Game/Assets/Buildings/Blue_Building.Blue_Building")
      (`self.SpawnParts`
        (:`true`
          (goto _label_2))
        (:`false`
          (set `self.id` 3))))
    (:`8`
      (`StaticMeshComponent.SetStaticMesh` _staticmesh "/Game/Assets/Buildings/GREEN_Building.GREEN_Building")
      (`self.SpawnParts`
        (:`true`
          (goto _label_2))
        (:`false`
          (set `self.id` 0))))
    (:`9`
      (goto _label))
    (:`10`
      (goto _label))
    (:`11`
      (goto _label))
    (:`12`
      (goto _label))
    (:`13`
      (goto _label))
    (:`14`
      (goto _label))))

(fn `RandomParts`
  (bind _staticmesh1 (`self.StaticMesh1`))
  (switch `int` (`KismetMathLibrary.RandomIntegerInRange` 0 3)
    (:`0`
      (`StaticMeshComponent.SetStaticMesh` _staticmesh1 "/Game/Assets/B_Parts/WatchTower_a.WatchTower_a"))
    (:`1`
      (`StaticMeshComponent.SetStaticMesh` _staticmesh1 "/Game/Assets/B_Parts/B_P_Groups/Fan_Group_a.Fan_Group_a"))
    (:`2`
      (`StaticMeshComponent.SetStaticMesh` _staticmesh1 "/Game/Assets/B_Parts/B_P_Groups/Vent_Group_a.Vent_Group_a"))))

(fn `UserConstructionScript`
  (`self.Random`))