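; Building spawner actor that creates a random building whenever an actor stops overlapping it.
; On end overlap, it picks one of three building classes at random and spawns it at the Start transform.
; Begin overlap only prints a spawn or don't-spawn message based on a comparison with Buildings, without gating the spawn.
; BeginPlay prints a debug greeting, and the Box end-overlap event is empty.
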(event `self.ReceiveBeginPlay`
  (`KismetSystemLibrary.PrintString` "Hello"))

(event `self.ReceiveActorBeginOverlap`
  (params (OtherActor :type "Actor Object Reference"))
  (if (== OtherActor "/Game/Blueprints/Buildings.Buildings")
    (`KismetSystemLibrary.PrintString` "dont spawn")
    (else
      (`KismetSystemLibrary.PrintString` "spawn"))))

(event `self.ReceiveTick`
  (params (DeltaSeconds :type "Float (single-precision)")))

(event `self.ReceiveActorEndOverlap`
  (params (OtherActor :type "Actor Object Reference"))
  (switch `int` (`KismetMathLibrary.RandomInteger` 3)
    (:`0`
      (`|SpawnActorFromClass` "/Game/Blueprints/Buildings.Buildings_C" (`self.start`) "Undefined" "OverrideRootScale"))
    (:`1`
      (`|SpawnActorFromClass` "/Game/Blueprints/Buildings2.Buildings2_C" (`self.start`) "Undefined" "OverrideRootScale"))
    (:`2`
      (`|SpawnActorFromClass` "/Game/Blueprints/Buildings3.Buildings3_C" (`self.start`) "Undefined" "OverrideRootScale"))))

(event `self.Box.OnComponentEndOverlap`
  (params (OtherActor :type "Actor Object Reference") (OtherComp :type "PrimitiveComponent Object Reference") (OtherBodyIndex :type Integer)))

(fn `UserConstructionScript`)