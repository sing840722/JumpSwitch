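; GM2 appears to be a game mode Blueprint that manages the high score screen and score-based difficulty.
; ShowScores toggles the HScoreWidget, calling GetScores to trigger OnStartUpRetrieve before creating it; a custom event pairs this toggle with UploadNewScore.
; Scoring converts score to a level and sets GameState_BP's FallingSpeed from that scaled level plus FixedSpeed.
; A write resetting the game state's Chance is left disconnected.
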(event `self.ReceiveBeginPlay`)

(event `CustomEvent_0`
  (`self.ShowScores`)
  (`self.UploadNewScore`))

(event `ShowScores`
  ;[1 1 1] Moses Happy placer
  (if (`self.isactive`)
    (`Widget.RemoveFromParent` (stale _returnvalue))
    (set `self.IsActive` false)
    (else
      (`self.GetScores`)
      (bind _returnvalue (`|CreateWidget` "/Game/UI/HScoreWidget.HScoreWidget_C" (`GameplayStatics.GetPlayerController` 0)))
      (`UserWidget.AddToViewport` _returnvalue 0)
      (set `self.IsActive` true))))

(event `GetScores`
  ;[1 1 1] Moses Happy placer
  (`self.OnStartUpRetrieve`))

(fn `Scoring`
  (params (Score :type "Float (double-precision)"))
  (bind _returnvalue (`self.ScoreToLevel` Score))
  (bind _asgame_state_bp (cast `/Game/Blueprints/GameState_BP` (`GameplayStatics.GetGameState`)))
  (set `/Game/Blueprints/GameState_BP.FallingSpeed` (+ (/ (`KismetMathLibrary.Conv_IntToDouble` _returnvalue) 4.5) (`/Game/Blueprints/GameState_BP.FixedSpeed` _asgame_state_bp)) _asgame_state_bp))

(fn `UserConstructionScript`)