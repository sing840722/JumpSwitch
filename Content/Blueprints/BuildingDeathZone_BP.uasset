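; BuildingDeathZone_BP is an overlap zone that recycles scrolling left and right building rows and ends the game when the player touches it.
; An overlapping building makes GameState_BP spawn the next one on the same side, then is removed from that side's array and destroyed if removal succeeds.
; An overlapping Player_Char opens the Defeat level.
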(event `self.ReceiveBeginPlay`)

(event `self.ReceiveActorBeginOverlap`
  (params (OtherActor :type "Actor Object Reference"))
  (bind _asleft_buildings_bp (cast `/Game/Blueprints/LeftBuildings_BP` OtherActor)
    (:`then`
      (bind _asgame_state_bp (cast `/Game/Blueprints/GameState_BP` (`GameplayStatics.GetGameState`)))
      (`/Game/Blueprints/GameState_BP.SpawnNextLeft` _asgame_state_bp)
      (bind _returnvalue (`KismetArrayLibrary.Array_RemoveItem` (`/Game/Blueprints/GameState_BP.LeftBuildingArray` _asgame_state_bp) _asleft_buildings_bp))
      (if _returnvalue
        (`self.K2_DestroyActor` _asleft_buildings_bp)))
    (:`CastFailed`
      (bind _asright_buildings_bp (cast `/Game/Blueprints/RightBuildings_BP` OtherActor)
        (:`then`
          (bind _asgame_state_bp_2 (cast `/Game/Blueprints/GameState_BP` (`GameplayStatics.GetGameState`)))
          (`/Game/Blueprints/GameState_BP.SpawnNextRight` _asgame_state_bp_2)
          (bind _returnvalue_2 (`KismetArrayLibrary.Array_RemoveItem` (`/Game/Blueprints/GameState_BP.RightBuildingArray` _asgame_state_bp_2) _asright_buildings_bp))
          (if _returnvalue_2
            (`self.K2_DestroyActor` _asright_buildings_bp)))
        (:`CastFailed`
          (cast `/Game/Blueprints/Player_Char` OtherActor)
          (`GameplayStatics.OpenLevel` "Defeat"))))))

(fn `UserConstructionScript`)