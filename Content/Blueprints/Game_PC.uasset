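; Player controller Blueprint that sets up the touch HUD and handles debug-style keyboard and tilt input.
; BeginPlay hides screen messages, adds the WButtonHud widget and enables touch interface and touch events.
; Number keys select CurrentColour, while B and M call ShowScores and CustomEvent0 on the GM2 game mode.
; Tilt only prints colour names; its nested branches repeat one condition, so only Green can print.
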(event `Key|B`
  (params (Key :type "Key Structure" :default "AnyKey"))
  (:`Pressed`
    (bind _asgm2 (cast `/Game/Blueprints/GM2` (`GameplayStatics.GetGameMode`)))
    (`/Game/Blueprints/GM2.ShowScores` _asgm2)))

(event `InputAxis|Tilt`
  (params (AxisValue :type "Float (single-precision)"))
  (bind _returnvalue_x (`KismetMathLibrary.BreakVector` (`self.GetInputVectorAxisValue`)))
  (if (< _returnvalue_x 0.0)
    (`KismetSystemLibrary.PrintString` "Set Green")
    (elif (< _returnvalue_x 0.0)
      (`KismetSystemLibrary.PrintString` "Set Yellow")
      (elif (< _returnvalue_x 0.0)
        (`KismetSystemLibrary.PrintString` "Set Red")
        (elif (< _returnvalue_x 0.0)
          (`KismetSystemLibrary.PrintString` "Set Blue"))))))

(event `Key|M`
  (params (Key :type "Key Structure" :default "AnyKey"))
  (:`Pressed`
    (bind _asgm2 (cast `/Game/Blueprints/GM2` (`GameplayStatics.GetGameMode`)))
    (`/Game/Blueprints/GM2.CustomEvent_0` _asgm2)))

(event `Key|One`
  (params (Key :type "Key Structure" :default "AnyKey"))
  (:`Pressed`
    (set `self.CurrentColour` 0)))

(event `Key|Two`
  (params (Key :type "Key Structure" :default "AnyKey"))
  (:`Pressed`
    (set `self.CurrentColour` 1)))

(event `Key|Three`
  (params (Key :type "Key Structure" :default "AnyKey"))
  (:`Pressed`
    (set `self.CurrentColour` 2)))

(event `Key|Four`
  (params (Key :type "Key Structure" :default "AnyKey"))
  (:`Pressed`
    (set `self.CurrentColour` 3)))

(event `self.ReceiveBeginPlay`
  (bind _returnvalue (`GameplayStatics.GetPlayerController` 0))
  (`KismetSystemLibrary.ExecuteConsoleCommand` "DisableAllScreenMessages")
  (bind _returnvalue_2 (`|CreateWidget` "/Game/Blueprints/wButtonHud.wButtonHud_C"))
  (`UserWidget.AddToViewport` _returnvalue_2 0)
  (`self.ActivateTouchInterface` _returnvalue null)
  (set `PlayerController.bEnableTouchEvents` true _returnvalue)
  (set `PlayerController.bEnableTouchOverEvents` true _returnvalue))

(event `self.ReceiveTick`
  (params (DeltaSeconds :type "Float (single-precision)")))

(fn `UserConstructionScript`)